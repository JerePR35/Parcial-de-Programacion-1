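; Player character BP_W for side-scrolling play, with Enhanced Input movement along world X, jump and dash.
; Horizontal velocity turns the controller yaw to face travel direction.
; Dash launches along the forward vector behind a delay-based cooldown, with a looping EndDash timer setting gravity scale.
; Walking off ledges opens a retriggerable coyote-time flag, which nothing here reads, and the CanJumpInternal override always returns false.
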(event Custom|EndDash
  ;[0.1468 0.02884 1] Dash
  (Variables|/Script/Engine.CharacterMovementComponent|SetGravityScale (Variables|Character|GetCharacterMovement) 1.5)
  (Utilities|Time|ClearTimerbyFunctionName 0 ""))

(event Input|EnhancedActionEvents|EnhancedInputActionIA_Movimiento
  (params (ActionValue :type Float%20%28double-precision%29) (ElapsedSeconds :type Float%20%28double-precision%29) (TriggeredSeconds :type Float%20%28double-precision%29) (InputAction :type Input%20Action%20Object%20Reference :default "/Game/Mapa/Imputs/IA_Movimiento.IA_Movimiento"))
  ;[0.1418 1 0.9203] Movimiento del personaje
  (Pawn|Input|AddMovementInput "1.000000,0.000000,0.000000" ActionValue false)
  (Math|Float|CompareFloat (.X (Math|Vector|BreakVector (Variables|/Script/Engine.MovementComponent|GetVelocity (Variables|Character|GetCharacterMovement)))) 0.0
    (:>
      (Pawn|SetControlRotation (Pawn|GetController) (Math|Rotator|MakeRotator 0.0 0.0 0.0)))
    (:<
      (Pawn|SetControlRotation (Pawn|GetController) (Math|Rotator|MakeRotator 0.0 0.0 1.8e+02)))))

(event Input|EnhancedActionEvents|EnhancedInputActionIA_Dash
  (params (ActionValue :type Boolean) (ElapsedSeconds :type Float%20%28double-precision%29) (TriggeredSeconds :type Float%20%28double-precision%29) (InputAction :type Input%20Action%20Object%20Reference :default "/Game/Mapa/Imputs/IA_Dash.IA_Dash"))
  ;[0.1468 0.02884 1] Dash
  (if (Variables|Dash|GetPuedehacerDash?)
    (Variables|Dash|SetPuedehacerDash? false)
    (Variables|/Script/Engine.CharacterMovementComponent|SetGravityScale (Variables|Character|GetCharacterMovement) 1.5)
    (Character|LaunchCharacter (* (Transformation|GetActorForwardVector) (Variables|Dash|GetVelocidad%20Dash)) true false)
    (Utilities|Time|SetTimerbyEvent (delegate Custom|EndDash) (Variables|Dash|GetTiempo%20en%20Dash) true true)
    (Utilities|FlowControl|Delay (Variables|Dash|GetTiempo%20para%20Volver%20a%20hacer%20Dash))
    (Variables|Dash|SetPuedehacerDash? true)))

(event Input|EnhancedActionEvents|EnhancedInputActionIA_Jump
  (params (ActionValue :type Boolean) (ElapsedSeconds :type Float%20%28double-precision%29) (TriggeredSeconds :type Float%20%28double-precision%29) (InputAction :type Input%20Action%20Object%20Reference :default "/Game/Mapa/Imputs/IA_Jump.IA_Jump"))
  ;[0.8337 0.3659 1] Salto del Personaje
  (:Triggered
    (Character|Jump))
  (:Completed
    (Character|StopJumping)))

(event EventOnWalkingOffLedge
  (params (PreviousFloorImpactNormal :type Vector%20%28by%20ref%29 :default "0, 0, 0") (PreviousFloorContactNormal :type Vector%20%28by%20ref%29 :default "0, 0, 0") (PreviousLocation :type Vector%20%28by%20ref%29 :default "0, 0, 0") (TimeDelta :type Float%20%28single-precision%29))
  ;[1 0.9229 0] Coyote Time
  (Development|PrintString "Hello")
  (Variables|CoyoteTime|SetIs%20in%20Coyote%20Time true)
  (Utilities|FlowControl|RetriggerableDelay (Variables|CoyoteTime|GetTiempo%20de%20Coyote))
  (Variables|CoyoteTime|SetIs%20in%20Coyote%20Time false))

(event EventBeginPlay
  ;[0.1812 1 0.273] Control del Personaje
  (bind _asplayer_controller (Utilities|Casting|CastToPlayerController (Pawn|GetController)))
  (Input|AddMappingContext (PlayerController|LocalPlayerSubsystems|GetEnhancedInputLocalPlayerSubsystem _asplayer_controller) "/Game/Mapa/Imputs/MapingContext/NewInputMappingContext.NewInputMappingContext" 0 "(bIgnoreAllPressedKeysUntilRelease=True,bForceImmediately=False,bNotifyUserSettings=False)"))

(fn ConstructionScript)

(fn CanJumpInternal
  (return false))